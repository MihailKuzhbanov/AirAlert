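; Light Scout enemy pawn that constantly moves forward while steering to face away from the player pawn, which it caches on BeginPlay.
; Each Tick, after the parent logic, it applies a fixed, unswept local forward offset that is not scaled by delta time.
; It then yaws toward the player-to-self direction, with the angle difference clamped by RotMaxSpeed and scaled by delta time.
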(event `self.ReceiveBeginPlay`
  (`parent.ReceiveBeginPlay`)
  (set `self.PawnBody` (`GameplayStatics.GetPlayerPawn` 0)))

(event `self.ReceiveTick`
  (params (DeltaSeconds :type "Float (single-precision)"))
  (bind _rotmaxspeed (`self.RotMaxSpeed`))
  (bind (_returnvalue_roll _returnvalue_pitch _returnvalue_yaw) (`KismetMathLibrary.BreakRotator` (`KismetMathLibrary.NormalizedDeltaRotator` (`KismetMathLibrary.FindLookAtRotation` (`self.K2_GetActorLocation` (`self.PawnBody`)) (`self.K2_GetActorLocation`)) (`self.K2_GetActorRotation`))))
  (`parent.ReceiveTick` DeltaSeconds)
  (`self.K2_AddActorLocalOffset` (3.0 0.0 0.0))
  (`self.K2_AddActorLocalRotation` (`KismetMathLibrary.MakeRotator` 0.0 0.0 (* (`KismetMathLibrary.FClamp` _returnvalue_yaw (* -1.0 _rotmaxspeed) _rotmaxspeed) (`GameplayStatics.GetWorldDeltaSeconds`)))))

(fn `UserConstructionScript`)